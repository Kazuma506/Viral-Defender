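; Melee virus enemy that wanders randomly, chases the player on sight, and can reproduce.
; Looping timers drive patrol and facing, while PawnSensing triggers AI moves ending in damage to active, ready antibodies or the player.
; Player hits teleport the virus randomly and open the Heart level at zero health.
; Laser overlaps damage it and may trigger a one-time, timeline-scaled split spawning a growing, non-reproducing copy.
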(event OnSeePawn(PawnSensing)
  (params (Pawn :type Pawn%20Object%20Reference))
  ;[1 1 1] Virus chase, virus reproduction and damage checks
  (bind _asfirst_person_character (Utilities|Casting|CastToFirstPerson_Character Pawn))
  (if (not (Variables|Default|GetbIsReproducing))
    (AI|AIMoveTo self (Transformation|GetActorLocation _asfirst_person_character) 0 1e+02 false
      (:OnSuccess
        (if (<= (Math|Vector|VectorLength (- (Transformation|GetActorLocation _asfirst_person_character) (Transformation|GetActorLocation (Game|GetPlayerCharacter 0)))) 93.0)
          (if (Variables|/Script/SNHU_FPS.FirstPerson_Character|GetbAntibodiesActive _asfirst_person_character)
            (bind _outactors (Actor|GetAllActorsOfClass "/Game/Mstew_Assets/Antibody_Handler.Antibody_Handler_C"))
            (for _array_element _outactors
              _)
            (if (Variables|/Game/Mstew_Assets/Antibody_Handler.Antibody_Handler_C|GetbAntibodiesReady _array_element)
              (Default|DamageTaken _array_element 1e+01)
              (else
                (CallFunction|DamageApplicationonPlayer :!label _label)
                (Utilities|FlowControl|MultiGate true false -1
                  (:Out%200
                    (Audio|PlaySound2D "/Game/Mstew_Assets/grunt1.grunt1"))
                  (:Out%201
                    (Audio|PlaySound2D "/Game/Mstew_Assets/grunt2.grunt2"))
                  (:Out%202
                    (Audio|PlaySound2D "/Game/Mstew_Assets/grunt3.grunt3"))
                  (:Out%203
                    (Audio|PlaySound2D "/Game/Mstew_Assets/grunt4.grunt4"))
                  (:Out%204
                    (Audio|PlaySound2D "/Game/Mstew_Assets/grunt5.grunt5"))
                  (:Out%205
                    (Audio|PlaySound2D "/Game/Mstew_Assets/grunt6.grunt6")))))
            (else
              (goto _label))))))))

(event OnComponentBeginOverlap(AI_Melee)
  (params (OverlappedComponent :type Primitive%20Component%20Object%20Reference) (OtherActor :type Actor%20Object%20Reference) (OtherComp :type Primitive%20Component%20Object%20Reference) (OtherBodyIndex :type Integer) (bFromSweep :type Boolean) (SweepResult :type Hit%20Result%20Structure%20%28by%20ref%29))
  ;[1 1 1] AI damage reciever
  (bind _asbp_laser (Utilities|Casting|CastToBP_Laser OtherActor))
  (Variables|Default|SetAI_Health (- (Variables|Default|GetAI_Health) 2e+01))
  (Actor|DestroyActor _asbp_laser)
  (if (<= (Variables|Default|GetAI_Health) 0.0)
    (Actor|DestroyActor)
    (elif (not (Variables|Default|GetbReproduced))
      (if (Math|Random|RandomBoolwithWeight 0.15)
        (Components|Movement|StopMovementImmediately (Variables|Character|GetCharacterMovement))
        (Variables|Default|SetbIsReproducing true)
        (CallFunction|Reproducing)))))

(event Custom|AI%20Patrol
  ;[1 1 1] AI Patrol, (Moves to random points in the Map)
  (if (not (Variables|Default|GetbIsReproducing))
    (Utilities|FlowControl|Delay (Math|Random|RandomFloatinRange 1.0 3.0))
    (AI|Navigation|SimpleMovetoLocation (Pawn|GetController) (AI|Navigation|GetRandomReachablePointinRadius (Transformation|GetActorLocation) 1e+03))))

(event Custom|Baby%20Grow
  ;[1 1 1] AI Growth after reproduction
  (bind _newtrack_2 (Timeline|Timeline_2 Play)
    (:Update
      (Transformation|SetActorScale3D _newtrack_2))
    (:Finished
      (Variables|Default|SetbIsReproducing false))))

(event Custom|Damage%20Application%20On%20Player
  ;[1 1 1] Damage Applier, and teleport feature
  (bind _asfirst_person_character (Utilities|Casting|CastToFirstPerson_Character (Game|Player|GetPlayerPawn 0)))
  (Variables|/Script/SNHU_FPS.FirstPerson_Character|Sethealth _asfirst_person_character (- (Variables|/Script/SNHU_FPS.FirstPerson_Character|Gethealth _asfirst_person_character) 1e+01))
  (Transformation|Teleport (AI|Navigation|GetRandomReachablePointinRadius (Transformation|GetActorLocation) 1e+03) "0, 0, 0")
  (if (<= (Variables|/Script/SNHU_FPS.FirstPerson_Character|Gethealth _asfirst_person_character) 0.0)
    (Game|OpenLevel(byName) "Heart")))

(event Custom|Rotate
  ;[1 1 1] Rotates the Melee Virus
  (Utilities|Casting|CastToFirstPerson_Character (Game|GetPlayerCharacter 0))
  (Transformation|SetActorRotation (Math|Rotator|FindLookatRotation (Transformation|GetActorLocation) (Transformation|GetActorLocation (Game|GetPlayerCharacter 0)))))

(event Custom|Distance
  ;[1 1 1] Distance De-bugger
  (Development|PrintString (Utilities|String|ToString(Float) (Math|Vector|VectorLength (- (Transformation|GetActorLocation (Game|GetPlayerCharacter 0)) (Transformation|GetActorLocation))))))

(event Custom|Reproducing
  ;[1 1 1] AI Reproduction
  (Variables|Default|SetbReproduced true)
  (bind _newtrack_0 (Timeline|Timeline_0 Play)
    (:Update
      (Transformation|SetActorScale3D _newtrack_0))
    (:Finished
      (bind _returnvalue (AI|SpawnAIFromClass "AI_Melee_BP_C" 0 (+ (Transformation|GetActorLocation) (Math|Vector|MakeVector (Math|Random|RandomFloatinRange -5e+01 -25.0) (Math|Random|RandomFloatinRange -5e+01 -25.0) 0.0)) "0, 0, 0" false))
      (bind _asai_melee_bp (Utilities|Casting|CastToAI_Melee_BP _returnvalue))
      (Variables|AI_Melee_BP_C|SetbReproduced _asai_melee_bp true)
      (CallFunction|BabyGrow _asai_melee_bp)
      (bind _newtrack_1 (Timeline|Timeline_1 Play)
        (:Update
          (Transformation|SetActorScale3D _newtrack_1))
        (:Finished
          (Variables|Default|SetbIsReproducing false))))))

(event EventBeginPlay
  ;[1 1 1] Function Calling
  (Utilities|Time|SetTimerbyFunctionName 0 "AI Patrol" 0.1 true)
  (Utilities|Time|SetTimerbyFunctionName 0 "Rotate" 1.0 true))

(fn ConstructionScript)