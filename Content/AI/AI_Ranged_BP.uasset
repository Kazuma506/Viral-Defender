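; AI_Ranged_BP is a stationary ranged enemy that shoots at the first-person player.
; Looping timers turn it to face the player and, while the player overlaps its Box, spawn projectiles from an Arrow with a sound.
; IsVisible reflects only that overlap, with no line-of-sight check.
; BP_Laser hits on the AI_Ranged component reduce health and destroy the laser, then the enemy once health runs out.
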(event OnComponentBeginOverlap(AI_Ranged)
  (params (OverlappedComponent :type Primitive%20Component%20Object%20Reference) (OtherActor :type Actor%20Object%20Reference) (OtherComp :type Primitive%20Component%20Object%20Reference) (OtherBodyIndex :type Integer) (bFromSweep :type Boolean) (SweepResult :type Hit%20Result%20Structure%20%28by%20ref%29))
  (bind _asbp_laser (Utilities|Casting|CastToBP_Laser OtherActor))
  (Variables|Default|SetAI%20Health (- (Variables|Default|GetAI%20Health) 1e+01))
  (Actor|DestroyActor _asbp_laser)
  (if (<= (Variables|Default|GetAI%20Health) 0.0)
    (Actor|DestroyActor)))

(event OnComponentBeginOverlap(Box)
  (params (OverlappedComponent :type Primitive%20Component%20Object%20Reference) (OtherActor :type Actor%20Object%20Reference) (OtherComp :type Primitive%20Component%20Object%20Reference) (OtherBodyIndex :type Integer) (bFromSweep :type Boolean) (SweepResult :type Hit%20Result%20Structure%20%28by%20ref%29))
  (Utilities|Casting|CastToFirstPerson_Character OtherActor)
  (Variables|Default|SetisVisible true))

(event OnComponentEndOverlap(Box)
  (params (OverlappedComponent :type Primitive%20Component%20Object%20Reference) (OtherActor :type Actor%20Object%20Reference) (OtherComp :type Primitive%20Component%20Object%20Reference) (OtherBodyIndex :type Integer))
  (Utilities|Casting|CastToFirstPerson_Character OtherActor)
  (Variables|Default|SetisVisible false))

(event Custom|Rotate
  (Transformation|SetActorRotation (Math|Rotator|FindLookatRotation (Transformation|GetActorLocation) (Transformation|GetActorLocation (Variables|Default|GetPlayerVar)))))

(event Custom|FIre
  (if (Variables|Default|GetisVisible)
    (Game|SpawnActorfromClass "/Game/AI/Projectile.Projectile_C" (Transformation|GetWorldTransform (Variables|Default|GetArrow)) "Undefined" 0 0)
    (Audio|PlaySound2D "/Game/ArtAssets/trink3.trink3" 2.5)))

(event EventBeginPlay
  (bind _asfirst_person_character (Utilities|Casting|CastToFirstPerson_Character (Game|Player|GetPlayerPawn 0)))
  (Variables|Default|SetPlayerVar _asfirst_person_character)
  (Utilities|Time|SetTimerbyFunctionName 0 "Rotate" 0.2 true)
  (Utilities|Time|SetTimerbyFunctionName 0 "Fire" 1.0 true))

(fn ConstructionScript)