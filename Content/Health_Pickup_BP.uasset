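; Rotating health pickup that respawns after being destroyed; the file itself contains no healing logic.
; On destruction it plays a sound and spawns a dormant replacement at its transform, which wakes after a ten-second BeginPlay delay.
; Tick hides dormant pickups and disables their collision.
; When active, Tick spins the actor and polls player health, showing a faded, non-collidable mesh at 100 health and a normal collidable one otherwise.
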(event EventTick
  (params (DeltaSeconds :type Float%20%28single-precision%29))
  (bind _staticmesh (Variables|Default|GetStaticMesh))
  (if (Variables|Default|GetbDormant)
    (Rendering|Material|SetMaterial _staticmesh 0 "/Game/ArtAssets/PickupInvisible.PickupInvisible")
    (Collision|SetCollisionEnabled _staticmesh "NoCollision")
    (else
      (Utilities|FlowControl|Sequence
        (:then_0
          (bind _asfirst_person_character (Utilities|Casting|CastToFirstPerson_Character (Game|Player|GetPlayerPawn 0)))
          (if (== (Variables|/Script/SNHU_FPS.FirstPerson_Character|Gethealth _asfirst_person_character) 1e+02)
            (Collision|SetCollisionEnabled (Variables|Default|GetStaticMesh) "NoCollision")
            (Rendering|Material|SetMaterial (Variables|Default|GetStaticMesh) 0 "/Game/ArtAssets/HealthPickupFaded.HealthPickupFaded")
            (else
              (Collision|SetCollisionEnabled (Variables|Default|GetStaticMesh) "QueryAndPhysics")
              (Rendering|Material|SetMaterial (Variables|Default|GetStaticMesh) 0 "/Game/ArtAssets/HealthPickup.HealthPickup"))))
        (:then_1
          (Transformation|AddActorLocalRotation (Math|Rotator|MakeRotator 0.0 0.0 (* DeltaSeconds (Variables|Default|GetYaw%20Rotation%20Per%20Second))) false false))))))

(event EventBeginPlay
  (Utilities|FlowControl|Delay 1e+01)
  (Variables|Default|SetbDormant false))

(event EventDestroyed
  (Audio|PlaySound2D "/Game/Mstew_Assets/healthpickup.healthpickup" 0.4)
  (bind _returnvalue (Game|SpawnActorfromClass "Health_Pickup_BP_C" (Transformation|GetActorTransform) "Undefined" 0 0))
  (Variables|Health_Pickup_BP_C|SetbDormant _returnvalue true))

(fn ConstructionScript)