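; BP_Portal5t4 is a one-way portal trigger that sends the first-person character to its partner, BP_Portal4t5.
; On BeginPlay it stores a reference to the BP_Portal4t5 found in the level.
; On character overlap it plays a sound, teleports the character there and matches control rotation to that portal.
; The destination's box overlap events are disabled during the jump and restored after a short delay, preventing an immediate bounce back.
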(event Collision|EventActorBeginOverlap
  (params (OtherActor :type Actor%20Object%20Reference))
  (bind _portal4t5 (Variables|Default|GetPortal4t5))
  (bind _asfirst_person_character (Utilities|Casting|CastToFirstPerson_Character OtherActor))
  (bind _asbp_portal_4t_5 (Utilities|Casting|CastToBP_Portal4t5 (Variables|Default|GetPortal4t5)))
  (Variables|/Script/Engine.PrimitiveComponent|SetbGenerateOverlapEvents (Variables|/Game/Mstew_Assets/BP_Portal4t5.BP_Portal4t5_C|GetBox _asbp_portal_4t_5) false)
  (Audio|PlaySound2D "/Game/Mstew_Assets/portalsound.portalsound")
  (Transformation|SetActorLocation _asfirst_person_character (Transformation|GetActorLocation _portal4t5) false true)
  (Pawn|SetControlRotation (Game|GetPlayerController 0) (Transformation|GetActorRotation _portal4t5))
  (Utilities|FlowControl|Delay 2.5)
  (Variables|/Script/Engine.PrimitiveComponent|SetbGenerateOverlapEvents (Variables|/Game/Mstew_Assets/BP_Portal4t5.BP_Portal4t5_C|GetBox _asbp_portal_4t_5) true))

(event EventBeginPlay
  (bind _outactors (Actor|GetAllActorsOfClass "/Game/Mstew_Assets/BP_Portal4t5.BP_Portal4t5_C"))
  (for _array_element _outactors
    (Variables|Default|SetPortal4t5 _array_element)))

(fn ConstructionScript)