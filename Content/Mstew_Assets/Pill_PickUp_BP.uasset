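; Antibody pill pickup that gives the player an attached Antibody_Handler, presumably a shield, when it is destroyed.
; On Destroyed it plays the Shield sound and spawns the handler on the character only if AntibodiesActive is set, which happens outside this graph.
; Tick polls that flag to disable collision and fade the material while antibodies are active.
; Tick also plays a timeline that moves the pill by local offsets.
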(event EventDestroyed
  (bind _returnvalue (Game|GetPlayerCharacter 0))
  (Audio|PlaySound2D "/Game/Mstew_Assets/shield.shield")
  (bind _asfirst_person_character (Utilities|Casting|CastToFirstPerson_Character _returnvalue))
  (if (Variables|/Script/SNHU_FPS.FirstPerson_Character|GetbAntibodiesActive _asfirst_person_character)
    (bind _returnvalue_2 (Game|SpawnActorfromClass "/Game/Mstew_Assets/Antibody_Handler.Antibody_Handler_C" (Math|Transform|MakeTransform (- (.Location (Math|Transform|BreakTransform (Transformation|GetActorTransform _returnvalue))) "0, 0,6.000000") "0, 0, 0" "1,1,1") "AlwaysSpawn" 0 0))
    (Transformation|AttachActorToActor _returnvalue_2 _returnvalue "None" "SnapToTarget" "KeepWorld" "KeepWorld" true)))

(event EventTick
  (params (DeltaSeconds :type Float%20%28single-precision%29))
  ;[1 1 1] Credit: Tesla Dev
  (Utilities|FlowControl|Sequence
    (:then_0
      (bind _asfirst_person_character (Utilities|Casting|CastToFirstPerson_Character (Game|Player|GetPlayerPawn 0)))
      (if (Variables|/Script/SNHU_FPS.FirstPerson_Character|GetbAntibodiesActive _asfirst_person_character)
        (Collision|SetCollisionEnabled (Variables|Default|GetStaticMesh) "NoCollision")
        (Rendering|Material|SetMaterial (Variables|Default|GetStaticMesh) 0 "/Game/ArtAssets/AntibodyPickupFaded.AntibodyPickupFaded")
        (else
          (Collision|SetCollisionEnabled (Variables|Default|GetStaticMesh) "QueryAndPhysics")
          (Rendering|Material|SetMaterial (Variables|Default|GetStaticMesh) 0 "/Game/ArtAssets/AntibodyPickup.AntibodyPickup"))))
    (:then_1
      (bind _vector (Timeline|Timeline_0 Play)
        (:Update
          (Transformation|AddActorLocalOffset _vector false false))))))

(fn ConstructionScript)