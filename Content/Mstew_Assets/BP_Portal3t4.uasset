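; BP_Portal3t4 is a key-gated portal that teleports the first-person character to a BP_Portal4t3.
; On BeginPlay it caches the last BP_Portal4t3 found as its destination.
; On overlap with Key set, it plays a sound, moves the character, matches control rotation, and disables the destination box's overlap events for a short delay.
; Without Key, it adds a new Key_Widget to the viewport.
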(event Collision|EventActorBeginOverlap
  (params (OtherActor :type Actor%20Object%20Reference))
  (bind _portal4t3 (Variables|Default|GetPortal4t3))
  (bind _asfirst_person_character (Utilities|Casting|CastToFirstPerson_Character OtherActor))
  (if (Variables|Default|GetKey?)
    (bind _asbp_portal_4t_3 (Utilities|Casting|CastToBP_Portal4t3 (Variables|Default|GetPortal4t3)))
    (Variables|/Script/Engine.PrimitiveComponent|SetbGenerateOverlapEvents (Variables|/Game/Mstew_Assets/BP_Portal4t3.BP_Portal4t3_C|GetBox _asbp_portal_4t_3) false)
    (Audio|PlaySound2D "/Game/Mstew_Assets/portalsound.portalsound")
    (Transformation|SetActorLocation _asfirst_person_character (Transformation|GetActorLocation _portal4t3) false true)
    (Pawn|SetControlRotation (Game|GetPlayerController 0) (Transformation|GetActorRotation _portal4t3))
    (Utilities|FlowControl|Delay 2.5)
    (Variables|/Script/Engine.PrimitiveComponent|SetbGenerateOverlapEvents (Variables|/Game/Mstew_Assets/BP_Portal4t3.BP_Portal4t3_C|GetBox _asbp_portal_4t_3) true)
    (else
      (bind _returnvalue (UserInterface|CreateWidget "/Game/Mstew_Assets/Key_Widget.Key_Widget_C"))
      (UserInterface|Viewport|AddtoViewport _returnvalue 0))))

(event EventBeginPlay
  (bind _outactors (Actor|GetAllActorsOfClass "/Game/Mstew_Assets/BP_Portal4t3.BP_Portal4t3_C"))
  (for _array_element _outactors
    (Variables|Default|SetPortal4t3 _array_element)))

(fn ConstructionScript)