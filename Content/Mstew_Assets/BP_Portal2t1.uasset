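; BP_Portal2t1 is a one-way teleporter that sends the first-person character to its paired BP_Portal1t2.
; On BeginPlay it finds the BP_Portal1t2 in the level and stores it as the destination.
; On overlap it plays a sound, teleports the character there and sets the controller to that portal's rotation.
; It disables overlap events on the destination's box for a short delay to prevent an immediate bounce back.
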(event Collision|EventActorBeginOverlap
  (params (OtherActor :type Actor%20Object%20Reference))
  (bind _portal1t2 (Variables|Default|GetPortal1t2))
  (bind _asfirst_person_character (Utilities|Casting|CastToFirstPerson_Character OtherActor))
  (bind _asbp_portal_1t_2 (Utilities|Casting|CastToBP_Portal1t2 (Variables|Default|GetPortal1t2)))
  (Variables|/Script/Engine.PrimitiveComponent|SetbGenerateOverlapEvents (Variables|/Game/Mstew_Assets/BP_Portal1t2.BP_Portal1t2_C|GetBox _asbp_portal_1t_2) false)
  (Audio|PlaySound2D "/Game/Mstew_Assets/portalsound.portalsound")
  (Transformation|SetActorLocation _asfirst_person_character (Transformation|GetActorLocation _portal1t2) false true)
  (Pawn|SetControlRotation (Game|GetPlayerController 0) (Transformation|GetActorRotation _portal1t2))
  (Utilities|FlowControl|Delay 2.5)
  (Variables|/Script/Engine.PrimitiveComponent|SetbGenerateOverlapEvents (Variables|/Game/Mstew_Assets/BP_Portal1t2.BP_Portal1t2_C|GetBox _asbp_portal_1t_2) true))

(event EventBeginPlay
  (bind _outactors (Actor|GetAllActorsOfClass "/Game/Mstew_Assets/BP_Portal1t2.BP_Portal1t2_C"))
  (for _array_element _outactors
    (Variables|Default|SetPortal1t2 _array_element)))

(fn ConstructionScript)