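; BP_Portal2t3 is a key-gated portal that teleports the first-person character to a BP_Portal3t2 actor found at BeginPlay.
; On overlap with Key set, it plays a sound, moves the character to the destination and matches control rotation to that portal.
; It disables overlap events on the destination's box for a short delay to prevent immediate re-triggering.
; Without the key, it shows Key_Widget instead.
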(event Collision|EventActorBeginOverlap
  (params (OtherActor :type Actor%20Object%20Reference))
  (bind _portal3t2 (Variables|Default|GetPortal3t2))
  (bind _asfirst_person_character (Utilities|Casting|CastToFirstPerson_Character OtherActor))
  (if (Variables|Default|GetKey?)
    (bind _asbp_portal_3t_2 (Utilities|Casting|CastToBP_Portal3t2 (Variables|Default|GetPortal3t2)))
    (Variables|/Script/Engine.PrimitiveComponent|SetbGenerateOverlapEvents (Variables|/Game/Mstew_Assets/BP_Portal3t2.BP_Portal3t2_C|GetBox _asbp_portal_3t_2) false)
    (Audio|PlaySound2D "/Game/Mstew_Assets/portalsound.portalsound")
    (Transformation|SetActorLocation _asfirst_person_character (Transformation|GetActorLocation _portal3t2) false true)
    (Pawn|SetControlRotation (Game|GetPlayerController 0) (Transformation|GetActorRotation _portal3t2))
    (Utilities|FlowControl|Delay 2.5)
    (Variables|/Script/Engine.PrimitiveComponent|SetbGenerateOverlapEvents (Variables|/Game/Mstew_Assets/BP_Portal3t2.BP_Portal3t2_C|GetBox _asbp_portal_3t_2) true)
    (else
      (bind _returnvalue (UserInterface|CreateWidget "/Game/Mstew_Assets/Key_Widget.Key_Widget_C"))
      (UserInterface|Viewport|AddtoViewport _returnvalue 0))))

(event EventBeginPlay
  (bind _outactors (Actor|GetAllActorsOfClass "/Game/Mstew_Assets/BP_Portal3t2.BP_Portal3t2_C"))
  (for _array_element _outactors
    (Variables|Default|SetPortal3t2 _array_element)))

(fn ConstructionScript)