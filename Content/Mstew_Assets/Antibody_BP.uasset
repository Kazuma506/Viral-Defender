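; Antibody actor that orbits the player character at a fixed horizontal radius, slightly raised above the character's location.
; Each Tick accumulates a rotation angle from RotationSpeed and delta time, then rotates an offset vector around the Z axis.
; It sets the actor transform to that offset added to player 0's location, with no attachment or other logic.
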(event EventTick
  (params (DeltaSeconds :type Float%20%28single-precision%29))
  (Variables|Default|SetCurrent%20Rotation (+ (* DeltaSeconds (Variables|Default|GetRotation%20Speed)) (Variables|Default|GetCurrent%20Rotation)))
  (Transformation|SetActorTransform (Math|Transform|MakeTransform (+ (Transformation|GetActorLocation (Game|GetPlayerCharacter 0)) (Math|Vector|RotateVectorAroundAxis "100.000000, 0, 0" (Variables|Default|GetCurrent%20Rotation) "0.000000,0.000000,1.000000") "0.000000,0.000000,20.000000") "0, 0, 0" "1,1,1")))

(fn ConstructionScript)