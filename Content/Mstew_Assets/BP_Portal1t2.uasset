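; BP_Portal1t2 is a key-gated portal that teleports the first-person character to the BP_Portal2t1 portal.
; On BeginPlay it finds and stores the destination portal, keeping the last instance found.
; On overlap with Key set, it plays a sound, moves the player and matches control rotation, disabling the destination's box overlaps for a short delay to prevent bouncing back.
; Without Key, it shows Key_Widget.
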(event Collision|EventActorBeginOverlap
  (params (OtherActor :type Actor%20Object%20Reference))
  (bind _portal2t1 (Variables|Default|GetPortal2t1))
  (bind _asfirst_person_character (Utilities|Casting|CastToFirstPerson_Character OtherActor))
  (if (Variables|Default|GetKey?)
    (bind _asbp_portal_2t_1 (Utilities|Casting|CastToBP_Portal2t1 (Variables|Default|GetPortal2t1)))
    (Variables|/Script/Engine.PrimitiveComponent|SetbGenerateOverlapEvents (Variables|/Game/Mstew_Assets/BP_Portal2t1.BP_Portal2t1_C|GetBox _asbp_portal_2t_1) false)
    (Audio|PlaySound2D "/Game/Mstew_Assets/portalsound.portalsound")
    (Transformation|SetActorLocation _asfirst_person_character (Transformation|GetActorLocation _portal2t1) false true)
    (Pawn|SetControlRotation (Game|GetPlayerController 0) (Transformation|GetActorRotation _portal2t1))
    (Utilities|FlowControl|Delay 2.5)
    (Variables|/Script/Engine.PrimitiveComponent|SetbGenerateOverlapEvents (Variables|/Game/Mstew_Assets/BP_Portal2t1.BP_Portal2t1_C|GetBox _asbp_portal_2t_1) true)
    (else
      (bind _returnvalue (UserInterface|CreateWidget "/Game/Mstew_Assets/Key_Widget.Key_Widget_C"))
      (UserInterface|Viewport|AddtoViewport _returnvalue 0))))

(event EventBeginPlay
  (bind _outactors (Actor|GetAllActorsOfClass "/Game/Mstew_Assets/BP_Portal2t1.BP_Portal2t1_C"))
  (for _array_element _outactors
    (Variables|Default|SetPortal2t1 _array_element)))

(fn ConstructionScript)