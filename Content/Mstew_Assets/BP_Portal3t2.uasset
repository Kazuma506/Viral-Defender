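; BP_Portal3t2 is a portal that teleports the first-person character to its paired BP_Portal2t3.
; On BeginPlay it finds that portal class in the level, keeping the last instance found.
; On overlap it plays a sound, moves the character there and matches player 0's control rotation to the destination.
; The destination's box overlap events are disabled for a short delay to prevent an immediate bounce back.
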(event Collision|EventActorBeginOverlap
  (params (OtherActor :type Actor%20Object%20Reference))
  (bind _portal2t3 (Variables|Default|GetPortal2t3))
  (bind _asfirst_person_character (Utilities|Casting|CastToFirstPerson_Character OtherActor))
  (bind _asbp_portal_2t_3 (Utilities|Casting|CastToBP_Portal2t3 (Variables|Default|GetPortal2t3)))
  (Variables|/Script/Engine.PrimitiveComponent|SetbGenerateOverlapEvents (Variables|/Game/Mstew_Assets/BP_Portal2t3.BP_Portal2t3_C|GetBox _asbp_portal_2t_3) false)
  (Audio|PlaySound2D "/Game/Mstew_Assets/portalsound.portalsound")
  (Transformation|SetActorLocation _asfirst_person_character (Transformation|GetActorLocation _portal2t3) false true)
  (Pawn|SetControlRotation (Game|GetPlayerController 0) (Transformation|GetActorRotation _portal2t3))
  (Utilities|FlowControl|Delay 2.5)
  (Variables|/Script/Engine.PrimitiveComponent|SetbGenerateOverlapEvents (Variables|/Game/Mstew_Assets/BP_Portal2t3.BP_Portal2t3_C|GetBox _asbp_portal_2t_3) true))

(event EventBeginPlay
  (bind _outactors (Actor|GetAllActorsOfClass "/Game/Mstew_Assets/BP_Portal2t3.BP_Portal2t3_C"))
  (for _array_element _outactors
    (Variables|Default|SetPortal2t3 _array_element)))

(fn ConstructionScript)