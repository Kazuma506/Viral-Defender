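; BP_Portal4t3 is a one-way teleporter that sends the first-person character to the BP_Portal3t4 actor in the level.
; On BeginPlay it finds and stores that partner portal.
; On overlap it plays a sound, moves the character to the partner's location and sets the controller's rotation to match the partner's.
; It disables the partner's box overlap events for a short delay to prevent an immediate bounce back.
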(event Collision|EventActorBeginOverlap
  (params (OtherActor :type Actor%20Object%20Reference))
  (bind _portal3t4 (Variables|Default|GetPortal3t4))
  (bind _asfirst_person_character (Utilities|Casting|CastToFirstPerson_Character OtherActor))
  (bind _asbp_portal_3t_4 (Utilities|Casting|CastToBP_Portal3t4 (Variables|Default|GetPortal3t4)))
  (Variables|/Script/Engine.PrimitiveComponent|SetbGenerateOverlapEvents (Variables|/Game/Mstew_Assets/BP_Portal3t4.BP_Portal3t4_C|GetBox _asbp_portal_3t_4) false)
  (Audio|PlaySound2D "/Game/Mstew_Assets/portalsound.portalsound")
  (Transformation|SetActorLocation _asfirst_person_character (Transformation|GetActorLocation _portal3t4) false true)
  (Pawn|SetControlRotation (Game|GetPlayerController 0) (Transformation|GetActorRotation _portal3t4))
  (Utilities|FlowControl|Delay 2.5)
  (Variables|/Script/Engine.PrimitiveComponent|SetbGenerateOverlapEvents (Variables|/Game/Mstew_Assets/BP_Portal3t4.BP_Portal3t4_C|GetBox _asbp_portal_3t_4) true))

(event EventBeginPlay
  (bind _outactors (Actor|GetAllActorsOfClass "/Game/Mstew_Assets/BP_Portal3t4.BP_Portal3t4_C"))
  (for _array_element _outactors
    (Variables|Default|SetPortal3t4 _array_element)))

(fn ConstructionScript)