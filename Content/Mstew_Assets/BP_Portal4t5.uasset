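; One-way link of a portal pair that teleports the first-person character from this portal to BP_Portal5t4.
; BeginPlay caches the destination actor by class search.
; On overlap with Key set, it plays a sound, moves the player and matches control rotation to the destination, disabling that portal's box overlaps for 2.5 seconds to avoid bouncing back.
; Without Key, it shows a key widget instead.
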(event Collision|EventActorBeginOverlap
  (params (OtherActor :type Actor%20Object%20Reference))
  (bind _portal5t4 (Variables|Default|GetPortal5t4))
  (bind _asfirst_person_character (Utilities|Casting|CastToFirstPerson_Character OtherActor))
  (if (Variables|Default|GetKey?)
    (bind _asbp_portal_5t_4 (Utilities|Casting|CastToBP_Portal5t4 (Variables|Default|GetPortal5t4)))
    (Variables|/Script/Engine.PrimitiveComponent|SetbGenerateOverlapEvents (Variables|/Game/Mstew_Assets/BP_Portal5t4.BP_Portal5t4_C|GetBox _asbp_portal_5t_4) false)
    (Audio|PlaySound2D "/Game/Mstew_Assets/portalsound.portalsound")
    (Transformation|SetActorLocation _asfirst_person_character (Transformation|GetActorLocation _portal5t4) false true)
    (Pawn|SetControlRotation (Game|GetPlayerController 0) (Transformation|GetActorRotation _portal5t4))
    (Utilities|FlowControl|Delay 2.5)
    (Variables|/Script/Engine.PrimitiveComponent|SetbGenerateOverlapEvents (Variables|/Game/Mstew_Assets/BP_Portal5t4.BP_Portal5t4_C|GetBox _asbp_portal_5t_4) true)
    (else
      (bind _returnvalue (UserInterface|CreateWidget "/Game/Mstew_Assets/Key_Widget.Key_Widget_C"))
      (UserInterface|Viewport|AddtoViewport _returnvalue 0))))

(event EventBeginPlay
  (bind _outactors (Actor|GetAllActorsOfClass "/Game/Mstew_Assets/BP_Portal5t4.BP_Portal5t4_C"))
  (for _array_element _outactors
    (Variables|Default|SetPortal5t4 _array_element)))

(fn ConstructionScript)